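; BP_StudyUECharacter is a character Blueprint that shows its health on an HP bar widget.
; On BeginPlay it casts its Widget component's user widget to WBP_HPbar, caches the widget and its HPBar, and sets the initial fill.
; The HPUpdate event refreshes the bar from GetHealth divided by MaxHealth; nothing in this graph calls it.
; Overlap, Tick and the construction script are empty.
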(event `self.ReceiveBeginPlay`
  (bind _aswbp_hpbar (cast `/Game/UI/WBP_HPbar` (`WidgetComponent.GetUserWidgetObject` (`self.Widget`))))
  (bind _output_get (set `self.As WBP HPbar` _aswbp_hpbar))
  (bind _output_get_2 (set `self.HP Bar` (`/Game/UI/WBP_HPbar.HP_Bar` _output_get)))
  (`ProgressBar.SetPercent` _output_get_2 (/ (`self.GetHealth`) (`self.MaxHealth`))))

(event `self.ReceiveActorBeginOverlap`
  (params (OtherActor :type "Actor Object Reference")))

(event `self.HPUpdate`
  (`ProgressBar.SetPercent` (`self.HP Bar`) (/ (`self.GetHealth`) (`self.MaxHealth`))))

(fn `UserConstructionScript`)